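; Player character Blueprint that keeps an overhead-style health widget in step with life, death, respawn and item pickup events.
; It binds those delegates on BeginPlay, and only the authority forwards them through Multy events, apparently multicasts.
; These show or hide the widget, set the UW_WorldPlayer life bar and value from CurrentLife, or display the taken item.
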(event Custom|onDeath_Event
  (params (Player :type Player%20Character%20Object%20Reference))
  (Networking|SwitchHasAuthority
    (:Authority
      (CallFunction|MultyonDeath))))

(event Custom|onRespawn_Event
  (params (Player :type Player%20Character%20Object%20Reference))
  (Networking|SwitchHasAuthority
    (:Authority
      (CallFunction|MultyonRespawn))))

(event Custom|onAddLife_Event
  (params (Player :type Player%20Character%20Object%20Reference) (damage :type Integer))
  (Networking|SwitchHasAuthority
    (:Authority
      (CallFunction|MultyAddLifeUI))))

(event Custom|Multy_OnDeath
  (Rendering|SetVisibility (Variables|Default|GetHealthBarWidget) false false))

(event Custom|Multy_AddLifeUI
  (CallFunction|UpdateLifeBar))

(event Custom|Multy_OnRespawn
  (Rendering|SetVisibility (Variables|Default|GetHealthBarWidget) true false)
  (CallFunction|UpdateLifeBar))

(event Custom|onAddItem_Event
  (params (Player :type Player%20Character%20Object%20Reference) (_item :type Item%20Structure))
  (Networking|SwitchHasAuthority
    (:Authority
      (CallFunction|MultyonAddItem _item))))

(event Custom|Multy_OnAddItem
  (params (Item :type Item%20Structure))
  (CallFunction|UpdateUIItemTake Item))

(event EventBeginPlay
  (EventDispatchers|AssignOnAddItem (delegate Custom|onAddItem_Event))
  (EventDispatchers|AssignOnDeath (delegate Custom|onDeath_Event))
  (EventDispatchers|AssignOnRespawn (delegate Custom|onRespawn_Event))
  (EventDispatchers|AssignOnAddLife (delegate Custom|onAddLife_Event))
  (CallFunction|UpdateLifeBar))

(event Collision|EventActorBeginOverlap
  (params (OtherActor :type Actor%20Object%20Reference)))

(event EventTick
  (params (DeltaSeconds :type Float%20%28single-precision%29)))

(fn ConstructionScript)

(fn UpdateLifeBar
  (bind _currentlife (Variables|Default|GetcurrentLife))
  (bind _asuw_world_player (Utilities|Casting|CastToUW_WorldPlayer (UserInterface|GetWidget (Variables|Default|GetHealthBarWidget))))
  (Progress|SetPercent (Variables|/Game/Blueprint/UI/World/UW_WorldPlayer.UW_WorldPlayer_C|GetLife_Bar _asuw_world_player) (/ _currentlife (Variables|Default|GetmaxLife)))
  (Variables|/Script/UMG.TextBlock|SetText (Variables|/Game/Blueprint/UI/World/UW_WorldPlayer.UW_WorldPlayer_C|GetLifeValue _asuw_world_player) (Utilities|Text|ToText(Float) (Math|Conversions|ToFloat(Integer) _currentlife) "HalfToEven")))

(fn UpdateUIItemTake
  (params (Item :type Item%20Structure))
  (bind _asuw_world_player (Utilities|Casting|CastToUW_WorldPlayer (UserInterface|GetWidget (Variables|Default|GetHealthBarWidget)))
    (:then
      (Default|ShowItemTake _asuw_world_player Item))
    (:CastFailed
      (Development|PrintString "NoUI" true true "(R=1.000000,G=0.000000,B=0.000000,A=1.000000)"))))