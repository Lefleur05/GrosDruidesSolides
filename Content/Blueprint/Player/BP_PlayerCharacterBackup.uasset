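; Player character Blueprint, named as a backup, that manages a floating health bar widget above game logic for life, death and respawn.
; Death and respawn events hide and show the widget component.
; Each Tick writes CurrentLife and its ratio to MaxLife into UW_TempLifeBar.
; Tick also tilts the widget toward player 0's viewpoint using look-at pitch and roll, with yaw locked at 180 degrees.
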(event Custom|onDeath_Event
  (params (Player :type Player%20Character%20Object%20Reference))
  (Rendering|SetVisibility (Variables|Default|GetHealthBarWidget_0) false false))

(event Custom|onRespawn_Event
  (params (Player :type Player%20Character%20Object%20Reference))
  (Rendering|SetVisibility (Variables|Default|GetHealthBarWidget_0) true false))

(event EventBeginPlay
  (EventDispatchers|AssignOnDeath (delegate Custom|onDeath_Event))
  (EventDispatchers|AssignOnRespawn (delegate Custom|onRespawn_Event)))

(event Collision|EventActorBeginOverlap
  (params (OtherActor :type Actor%20Object%20Reference)))

(event EventTick
  (params (DeltaSeconds :type Float%20%28single-precision%29))
  (bind _returnvalue (Game|GetPlayerController 0))
  (bind _currentlife (Variables|Default|GetcurrentLife))
  (bind _healthbarwidget_0 (Variables|Default|GetHealthBarWidget_0))
  (bind _location (Pawn|GetPlayerViewPoint _returnvalue))
  (bind _returnvalue_2 (Transformation|GetWorldLocation _healthbarwidget_0))
  (bind _returnvalue_3 (Math|Rotator|FindLookatRotation _returnvalue_2 _location))
  (Utilities|FlowControl|Sequence
    (:then_0
      (bind _asuw_temp_life_bar (Utilities|Casting|CastToUW_TempLifeBar (UserInterface|GetWidget (Variables|Default|GetHealthBarWidget_0))))
      (Progress|SetPercent (Variables|/Game/Blueprint/UI/Temp/UW_TempLifeBar.UW_TempLifeBar_C|GetLife_Bar _asuw_temp_life_bar) (/ _currentlife (Variables|Default|GetmaxLife)))
      (Variables|/Script/UMG.TextBlock|SetText (Variables|/Game/Blueprint/UI/Temp/UW_TempLifeBar.UW_TempLifeBar_C|GetLifeValue _asuw_temp_life_bar) (Utilities|Text|ToText(Float) _currentlife "HalfToEven")))
    (:then_1
      (Transformation|SetWorldRotation _healthbarwidget_0 (Math|Rotator|MakeRotator (.roll _returnvalue_3) (.pitch _returnvalue_3) 1.8e+02) false false))))

(fn ConstructionScript)