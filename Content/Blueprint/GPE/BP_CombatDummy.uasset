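; Combat dummy actor that shows its health and pops up a damage number when its life changes.
; A world-space player widget displays the life bar and value, initialized shortly after BeginPlay.
; The life-change delegate triggers, on authority only, a Multy_AddLife event that refreshes the widget.
; That event also has the authority spawn a BP_DamageUI actor at the health bar with the absolute amount.
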(event Custom|onDummyAddLife_Event
  (params (combatDummy :type Combat%20Dummy%20Object%20Reference) (damage :type Float%20%28single-precision%29))
  (Networking|SwitchHasAuthority
    (:Authority
      (CallFunction|MultyAddLife damage))))

(event Custom|Multy_AddLife
  (params (damage :type Float%20%28double-precision%29))
  (CallFunction|UpdateUILife)
  (Networking|SwitchHasAuthority
    (:Authority
      (CallFunction|SpawnDamageUI damage))))

(event EventBeginPlay
  (Utilities|FlowControl|Sequence
    (:then_0
      (bind _asuw_world_player (Utilities|Casting|CastToUW_WorldPlayer (UserInterface|GetWidget (Variables|Default|GetHealthBarWidget))))
      (Widget|SetVisibility (Variables|/Game/Blueprint/UI/World/UW_WorldPlayer.UW_WorldPlayer_C|GetLifeValue _asuw_world_player) "Visible"))
    (:then_1
      (EventDispatchers|AssignOnDummyAddLife (delegate Custom|onDummyAddLife_Event))
      (Utilities|FlowControl|Delay 1.0)
      (CallFunction|UpdateUILife))))

(event Collision|EventActorBeginOverlap
  (params (OtherActor :type Actor%20Object%20Reference)))

(event EventTick
  (params (DeltaSeconds :type Float%20%28single-precision%29)))

(fn ConstructionScript)

(fn SpawnDamageUI
  (params (Damage :type Float%20%28double-precision%29))
  (bind _healthbarwidget (Variables|Default|GetHealthBarWidget))
  (bind _returnvalue (Transformation|GetWorldTransform _healthbarwidget))
  (Game|SpawnActorfromClass "/Game/Blueprint/GPE/BP_DamageUI.BP_DamageUI_C" (Math|Transform|MakeTransform (.location _returnvalue) (.rotation _returnvalue) (.scale _returnvalue)) "AlwaysSpawn" "MultiplyWithRoot" 0 (Math|Float|Absolute(Float) Damage) 0))

(fn UpdateUILife
  (bind _asuw_world_player (Utilities|Casting|CastToUW_WorldPlayer (UserInterface|GetWidget (Variables|Default|GetHealthBarWidget))))
  (Progress|SetPercent (Variables|/Game/Blueprint/UI/World/UW_WorldPlayer.UW_WorldPlayer_C|GetLife_Bar _asuw_world_player) (/ (Variables|Default|GetcurrentLife) (Variables|Default|GetmaxLife)))
  (Variables|/Script/UMG.TextBlock|SetText (Variables|/Game/Blueprint/UI/World/UW_WorldPlayer.UW_WorldPlayer_C|GetLifeValue _asuw_world_player) (Utilities|Text|ToText(Float) (Variables|Default|GetcurrentLife) "HalfToEven")))