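; BP_DamageUI is a short-lived floating damage number actor that shows a damage value through a widget component.
; On BeginPlay it passes its Damage value to the WBP_DamageAmount widget.
; With authority only, a timeline lerps the actor from its spawn point to a raised world-space offset with randomized Y drift, then destroys it.
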(event EventBeginPlay
  (bind _aswbp_damage_amount (Utilities|Casting|CastToWBP_DamageAmount (UserInterface|GetWidget (Variables|Default|GetWidget))))
  (Variables|/Game/Blueprint/UI/World/WBP_DamageAmount.WBP_DamageAmount_C|SetDamageAmount _aswbp_damage_amount (Variables|Default|Getdamage))
  (Networking|SwitchHasAuthority
    (:Authority
      (bind _output_get (Variables|Default|SetStartLocation (Transformation|GetActorLocation)))
      (Variables|Default|SetEndLocation (+ _output_get (Math|Vector|MakeVector 1.1e+02 (Math|Random|RandomFloatinRange -2e+02 2e+02) 1.2e+02)))
      (bind _move_track (Timeline|Timeline Play)
        (:Update
          (Transformation|SetActorLocation (Math|Vector|Lerp(Vector) (Variables|Default|GetStartLocation) (Variables|Default|GetEndLocation) _move_track) false false))
        (:Finished
          (Actor|DestroyActor))))))

(event Collision|EventActorBeginOverlap
  (params (OtherActor :type Actor%20Object%20Reference)))

(event EventTick
  (params (DeltaSeconds :type Float%20%28single-precision%29)))

(fn ConstructionScript)