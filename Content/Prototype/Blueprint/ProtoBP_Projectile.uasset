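; Prototype spell projectile that damages and knocks back players other than its caster.
; Construction applies speed and clamped scale from Stats, plus a material.
; Box overlap hits players and, with CancelSpell, destroys other players' projectiles; Tick detonates it once past its range.
; Explode sphere-traces to damage and launch each character once, caster included, with knockback velocities derived from braking deceleration.
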(event OnComponentBeginOverlap(Box)
  (params (OverlappedComponent :type Primitive%20Component%20Object%20Reference) (OtherActor :type Actor%20Object%20Reference) (OtherComp :type Primitive%20Component%20Object%20Reference) (OtherBodyIndex :type Integer) (bFromSweep :type Boolean) (SweepResult :type Hit%20Result%20Structure%20%28by%20ref%29))
  (bind _stats (Variables|Default|GetStats))
  ;[0.04606 0.1261 0.15 0.5 66] Lorsque le projectile touche un joueur ou un autre projectile
  (if (.cancelspell? (Variables|Default|GetStats))
    (bind _asbp_projectile (Utilities|Casting|CastToProtoBP_Projectile OtherActor)
      (:then
        (if (== (Variables|/Game/Prototype/ThirdPerson/Blueprints/ProtoBP_ThirdPersonCharacter.ProtoBP_ThirdPersonCharacter_C|GetID_Player (Variables|ProtoBP_Projectile_C|GetCaster _asbp_projectile)) (Variables|/Game/Prototype/ThirdPerson/Blueprints/ProtoBP_ThirdPersonCharacter.ProtoBP_ThirdPersonCharacter_C|GetID_Player (Variables|Default|GetCaster)))
          _
          (else
            (Actor|DestroyActor _asbp_projectile))))
      (:CastFailed
        _)))
  (bind _asproto_bp_third_person_character (Utilities|Casting|CastToProtoBP_ThirdPersonCharacter OtherActor))
  (if (not (== (Variables|/Game/Prototype/ThirdPerson/Blueprints/ProtoBP_ThirdPersonCharacter.ProtoBP_ThirdPersonCharacter_C|GetID_Player _asproto_bp_third_person_character) (Variables|/Game/Prototype/ThirdPerson/Blueprints/ProtoBP_ThirdPersonCharacter.ProtoBP_ThirdPersonCharacter_C|GetID_Player (Variables|Default|GetCaster))))
    (if (> (.knockback _stats) 0)
      (CallFunction|Knockback _asproto_bp_third_person_character))
    (Default|HPModifier _asproto_bp_third_person_character (* (.damages _stats) -1.0) self)
    (CallFunction|Explode)
    (Components|DestroyComponent (Variables|Default|GetBox))
    (Utilities|FlowControl|Delay 0.05)
    (Actor|DestroyActor)))

(event EventBeginPlay
  ;[0.15 0.15 0.15 0.5] Set la position initiale du projectile
  (Variables|Default|SetCurrentLocation (Transformation|GetActorLocation)) ; Nécessaire pour le calcul de la portée du projectile
)

(event EventTick
  (params (DeltaSeconds :type Float%20%28single-precision%29))
  ;[0.15 0.15 0.15 0.5 50] Calcul de la portée d'un sort
  (bind _output_get (Variables|Default|SetCurrentDistance (Math|Float|Absolute(Float) (Math|Vector|Distance(Vector) (Variables|Default|GetCurrentLocation) (Transformation|GetActorLocation)))))
  (if (>= _output_get (.range (Variables|Default|GetStats)))
    (CallFunction|Explode)
    (Actor|DestroyActor)))

(fn ConstructionScript
  (bind _projectilemovement (Variables|Default|GetProjectileMovement))
  (bind _stats (Variables|Default|GetStats))
  (bind _returnvalue (Math|Conversions|ToFloat(Integer) (.projectilespeed _stats)))
  (Variables|/Script/Engine.ProjectileMovementComponent|SetInitialSpeed _projectilemovement _returnvalue)
  (Variables|/Script/Engine.ProjectileMovementComponent|SetMaxSpeed _projectilemovement _returnvalue)
  (Rendering|Material|SetMaterial (Variables|Default|GetProjectileMesh) 0 (Variables|Default|GetMaterialToUse))
  (Transformation|SetActorScale3D (Math|Vector|MakeVector (Math|Float|Clamp(Float) (.x (.size _stats)) 0.5 1e+01) (Math|Float|Clamp(Float) (.y (.size _stats)) 0.5 1e+01) (Math|Float|Clamp(Float) (.z (.size _stats)) 0.5 8.0))))

(fn Knockback
  (params (PlayerHit :type Proto%20BP%20Third%20Person%20Character%20Object%20Reference))
  (Character|Jump PlayerHit)
  (Character|LaunchCharacter PlayerHit (* (Math|Vector|GetForwardVector (Variables|Default|GetArrowForward)) (Math|Float|Sqrt (* (.knockback (Variables|Default|GetStats)) (Variables|/Script/Engine.CharacterMovementComponent|GetBrakingDecelerationWalking (Variables|/Script/Engine.Character|GetCharacterMovement PlayerHit)) 1e+02 2.0))) false false))

(fn Explode
  (bind _returnvalue (Transformation|GetActorLocation))
  (bind _stats (Variables|Default|GetStats))
  (if (> (.explosionsize _stats) 0.0)
    (bind _outhits (Collision|MultiSphereTraceByChannel _returnvalue _returnvalue (.explosionsize _stats) "TraceTypeQuery3" false 0 "ForDuration" true "(R=0.401042,G=0.234524,B=0.218609,A=0.669565)" "(R=1.000000,G=0.191304,B=0.000000,A=1.000000)" 1.5))
    (for _array_element _outhits
      (bind _asproto_bp_third_person_character (Utilities|Casting|CastToProtoBP_ThirdPersonCharacter (.HitActor (Collision|BreakHitResult _array_element))))
      (if (== (Utilities|Array|FindItem (Variables|Default|GetHitPlayers) _asproto_bp_third_person_character) -1)
        (Utilities|Array|AddUnique (Variables|Default|GetHitPlayers) _asproto_bp_third_person_character)
        (Character|LaunchCharacter _asproto_bp_third_person_character (* (Math|Vector|Normalize (- (Transformation|GetActorLocation _asproto_bp_third_person_character) (.Location (Collision|BreakHitResult _array_element))) 1.0) (Math|Float|Sqrt (* (Variables|/Script/Engine.CharacterMovementComponent|GetBrakingDecelerationWalking (Variables|/Script/Engine.Character|GetCharacterMovement _asproto_bp_third_person_character)) 2.0 (* (.knockback _stats) 150)))) true true)
        (Default|HPModifier _asproto_bp_third_person_character (* (.explosiondamage _stats) -1.0) self)))
    (Utilities|Array|Clear (Variables|Default|GetHitPlayers))))