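; Prototype blade hazard that damages a ProtoBP_ThirdPersonCharacter when it begins overlapping the actor.
; It passes the negated Damages value to the character's HPModifier.
; A switch on IDPlayer gives each of four players a separate boolean gate, reset by a short Delay, so repeat overlaps are throttled per player.
; Damage comes only from begin-overlap events, so staying inside the blades does not tick further damage.
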(event EventBeginPlay)

(event Collision|EventActorBeginOverlap
  (params (OtherActor :type Actor%20Object%20Reference))
  (bind _asproto_bp_third_person_character (Utilities|Casting|CastToProtoBP_ThirdPersonCharacter OtherActor))
  (switch int (Variables|/Game/Prototype/ThirdPerson/Blueprints/ProtoBP_ThirdPersonCharacter.ProtoBP_ThirdPersonCharacter_C|GetID_Player _asproto_bp_third_person_character)
    (:0
      (if (Variables|Default|GetDelay1)
        (Variables|Default|SetDelay1 false)
        (Default|HPModifier _asproto_bp_third_person_character (* (Variables|Default|GetDamages) -1.0))
        (Utilities|FlowControl|Delay 0.2)
        (Variables|Default|SetDelay1 true)))
    (:1
      (if (Variables|Default|GetDelay2)
        (Variables|Default|SetDelay2 false)
        (Default|HPModifier _asproto_bp_third_person_character (* (Variables|Default|GetDamages) -1.0))
        (Utilities|FlowControl|Delay 0.2)
        (Variables|Default|SetDelay2 true)))
    (:2
      (if (Variables|Default|GetDelay3)
        (Variables|Default|SetDelay3 false)
        (Default|HPModifier _asproto_bp_third_person_character (* (Variables|Default|GetDamages) -1.0))
        (Utilities|FlowControl|Delay 0.2)
        (Variables|Default|SetDelay3 true)))
    (:3
      (if (Variables|Default|GetDelay4)
        (Variables|Default|SetDelay4 false)
        (Default|HPModifier _asproto_bp_third_person_character (* (Variables|Default|GetDamages) -1.0))
        (Utilities|FlowControl|Delay 0.2)
        (Variables|Default|SetDelay4 true)))))

(event EventTick
  (params (DeltaSeconds :type Float%20%28single-precision%29)))

(fn ConstructionScript)