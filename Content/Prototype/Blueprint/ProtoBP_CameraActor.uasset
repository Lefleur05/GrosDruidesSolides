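; Prototype shared camera actor that keeps multiple players in frame by following and zooming on them.
; BeginPlay gathers the player characters and centers the actor on their average location.
; Each Tick finds the farthest-apart pair, lerps toward their offset midpoint, and maps their distance to spring arm length, with a shortcut for two or fewer players.
; An older centroid-based version remains as unconnected nodes.
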(event Custom|MoveCameraForAllPlayers
  (bind _players (Variables|Default|GetPlayers))
  (bind _players_2 (Variables|Default|GetPlayers))
  (bind _returnvalue (Utilities|Array|Length _players))
  ;[0.6875 0.1217 0.5446 0.5 60] Set up du suivi de la caméra
  (for _index (range 0 (- _returnvalue 2)) ; On récupère les paires du joueur 1 au joueur 4
    (for _index_2 (range (+ _index 1) (- _returnvalue 1)) ; Récupérer la paire par rapport au joueur précédent
      (if (> (Math|Vector|Distance(Vector) (Transformation|GetActorLocation (Utilities|Array|Get(acopy) _players_2 _index)) (Transformation|GetActorLocation (Utilities|Array|Get(acopy) _players_2 _index_2))) (Variables|Default|GetMaxDistance)) ; On vérifie si la paire de joueurs a la distance la plus élevée
        (Variables|Default|SetMaxDistance (Math|Vector|Distance(Vector) (Transformation|GetActorLocation (Utilities|Array|Get(acopy) _players_2 _index)) (Transformation|GetActorLocation (Utilities|Array|Get(acopy) _players_2 _index_2)))) ; On définit la distance maximale
        (Variables|Default|SetPlayer_A (Utilities|Array|Get(acopy) _players_2 _index)) ; On définit l'un des joueurs les plus éloignés
        (Variables|Default|SetPlayer_B (Utilities|Array|Get(acopy) _players_2 _index_2)) ; On définit l'autre joueur le plus éloigné
      )))
  (Transformation|SetActorLocation (Math|Vector|Lerp(Vector) (Variables|Default|GetPositionBeforeLerp) (* (+ (+ (Transformation|GetActorLocation (Variables|Default|GetPlayer_A)) (Transformation|GetActorLocation (Variables|Default|GetPlayer_B))) "200.000000,0.000000,0.000000") 0.5) 0.25) false false) ; Placer la caméra entre les 2 joueurs
  (Variables|/Script/Engine.SpringArmComponent|SetTargetArmLength (Variables|Default|GetSpringArm) (* (Math|Float|MapRangeClamped (Variables|Default|GetMaxDistance) (Variables|Tuto|GetMinDistanceFromCenterPoint) (Variables|Tuto|GetMaxDistanceFromCenterPoint) (Variables|Tuto|GetMinZoom) (Variables|Tuto|GetMaxZoom)) (Variables|Tuto|GetMinDistance))))

(event Custom|MoveCameraForTwoPlayers
  (bind _players (Variables|Default|GetPlayers))
  (bind _output (Utilities|Array|Get(acopy) _players 1))
  ;[0.6875 0.1217 0.5446 0.5 60] Set up du suivi de la caméra
  (bind _output_get (Variables|Default|SetPlayer_A (Utilities|Array|Get(acopy) _players)))
  (Utilities|IsValid _output
    (:Is%20Valid
      (bind _output_get_2 (Variables|Default|SetPlayer_B _output)))
    (:Is%20Not%20Valid
      _))
  (Variables|Default|SetMaxDistance (Math|Vector|Distance(Vector) (Transformation|GetActorLocation _output_get) (Transformation|GetActorLocation _output_get_2)))
  (Transformation|SetActorLocation (Math|Vector|Lerp(Vector) (Variables|Default|GetPositionBeforeLerp) (* (+ (+ (Transformation|GetActorLocation (Variables|Default|GetPlayer_A)) (Transformation|GetActorLocation (Variables|Default|GetPlayer_B))) "200.000000,0.000000,0.000000") 0.5) 0.25) false false) ; Placer la caméra entre les 2 joueurs
  (Variables|/Script/Engine.SpringArmComponent|SetTargetArmLength (Variables|Default|GetSpringArm) (* (Math|Float|MapRangeClamped (Variables|Default|GetMaxDistance) (Variables|Tuto|GetMinDistanceFromCenterPoint) (Variables|Tuto|GetMaxDistanceFromCenterPoint) (Variables|Tuto|GetMinZoom) (Variables|Tuto|GetMaxZoom)) (Variables|Tuto|GetMinDistance))))

(event EventTick
  (params (DeltaSeconds :type Float%20%28single-precision%29))
  ;[0.6875 0.1217 0.5446 0.5 60] Set up du suivi de la caméra
  (if (Variables|Default|GetcanTick)
    (Variables|Default|SetPositionBeforeLerp (Transformation|GetActorLocation))
    (Variables|Default|SetMaxDistance 0.0)
    (if (> (Utilities|Array|Length (Variables|Default|GetPlayers)) 2)
      (CallFunction|MoveCameraforAllPlayers)
      (else
        (CallFunction|MoveCameraforTwoPlayers)))))

(event EventBeginPlay
  ;[0.15 0.1181 0.0278 0.5 80] Positionner la caméra et déterminer le nombre de joueurs
  (bind _returnvalue (Class|GameModeBase|GetNumPlayers (Game|GetGameMode)))
  (Variables|Tuto|SetLocationsSum "0, 0, 0")
  (for _index (range 0 (- _returnvalue 1))
    (bind _asproto_bp_third_person_character (Utilities|Casting|CastToProtoBP_ThirdPersonCharacter (Game|GetPlayerCharacter _index)))
    (Variables|Tuto|SetLocationsSum (+ (Variables|Tuto|GetLocationsSum) (Transformation|GetActorLocation _asproto_bp_third_person_character)))
    (Utilities|Array|AddUnique (Variables|Default|GetPlayers) _asproto_bp_third_person_character))
  (Transformation|SetActorLocation (/ (Variables|Tuto|GetLocationsSum) _returnvalue) false false)
  (Variables|Default|SetcanTick true))

(fn ConstructionScript)