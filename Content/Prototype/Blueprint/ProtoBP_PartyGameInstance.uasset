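; Party game instance that carries player stats, items and free-for-all scores between rounds and plays background music.
; Save events append each player's projectile stats, health, speed, dash cooldown and current item (four item slots) to arrays.
; WinConditionFFA shows the victory points widget; at three points it clears saved data, resets rankings and returns to the main menu after a delay.
; Init starts a random persistent track, but its replay-on-finish binding is unconnected.
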(event Custom|BaseRankPlayers
  (params (Players :type Array%20of%20Proto%20BP%20Third%20Person%20Character%20Object%20References))
  ;[0.15 0.15 0.15 0.5 74] Sauvegarder les statistiques
  (if (not (Variables|Default|GetneedRankPlayers))
    (for _array_element Players
      (Utilities|Array|Add (Variables|Default|GetRankingPlayers) 0))
    (Variables|Default|SetneedRankPlayers true)))

(event Custom|SaveStats
  (params (Players :type Array%20of%20Proto%20BP%20Third%20Person%20Character%20Object%20References))
  (bind _statsplayers (Variables|Players|GetStatsPlayers))
  ;[0.15 0.15 0.15 0.5 74] Sauvegarder les statistiques
  (Variables|Players|SetPlayers Players)
  (for _array_element Players ; Créer une liste de stats
    (Utilities|Array|Add _statsplayers (Variables|/Game/Prototype/ThirdPerson/Blueprints/ProtoBP_ThirdPersonCharacter.ProtoBP_ThirdPersonCharacter_C|GetST_PrimaryProjectile _array_element))
    (Utilities|Array|Add _statsplayers (Variables|/Game/Prototype/ThirdPerson/Blueprints/ProtoBP_ThirdPersonCharacter.ProtoBP_ThirdPersonCharacter_C|GetST_SecondaryProjectile _array_element))
    (Utilities|Array|Add _statsplayers (Variables|/Game/Prototype/ThirdPerson/Blueprints/ProtoBP_ThirdPersonCharacter.ProtoBP_ThirdPersonCharacter_C|GetST_UtilitaryProjectile _array_element))
    (Utilities|Array|Add _statsplayers (Variables|/Game/Prototype/ThirdPerson/Blueprints/ProtoBP_ThirdPersonCharacter.ProtoBP_ThirdPersonCharacter_C|GetST_UltimateProjectile _array_element))
    (Utilities|Array|Add (Variables|Players|GetPlayerHP) (Variables|/Game/Prototype/ThirdPerson/Blueprints/ProtoBP_ThirdPersonCharacter.ProtoBP_ThirdPersonCharacter_C|GetMax_HealthPoints _array_element))
    (Utilities|Array|Add (Variables|Players|GetPlayerSpeed) (Variables|/Script/Engine.CharacterMovementComponent|GetMaxWalkSpeed (Variables|/Script/Engine.Character|GetCharacterMovement _array_element)))
    (Utilities|Array|Add (Variables|Players|GetPlayerDashCD) (Variables|/Game/Prototype/ThirdPerson/Blueprints/ProtoBP_ThirdPersonCharacter.ProtoBP_ThirdPersonCharacter_C|GetDashCooldown _array_element))))

(event Custom|EndGame
  (Utilities|FlowControl|Delay 8.0)
  (Game|OpenLevel(byName) "LVL_MainMenu"))

(event Custom|RoundFinish
  ;[0.7196 0.7396 0.2234 0.5 98] Fin de round
)

(event Custom|Save%20Items
  (params (Players :type Array%20of%20Proto%20BP%20Third%20Person%20Character%20Object%20References))
  ;[0.15 0.15 0.15 0.5 74] Sauvegarder les statistiques
  (for (_array_element _array_index) Players
    (switch int _array_index
      (:0
        (Utilities|Array|Add (Variables|Players|GetPlayer1_ItemsSlots) (Variables|/Game/Prototype/ThirdPerson/Blueprints/ProtoBP_ThirdPersonCharacter.ProtoBP_ThirdPersonCharacter_C|GetCurrentItem _array_element)))
      (:1
        (Utilities|Array|Add (Variables|Players|GetPlayer2_ItemsSlots) (Variables|/Game/Prototype/ThirdPerson/Blueprints/ProtoBP_ThirdPersonCharacter.ProtoBP_ThirdPersonCharacter_C|GetCurrentItem _array_element)))
      (:2
        (Utilities|Array|Add (Variables|Players|GetPlayer3_ItemsSlots) (Variables|/Game/Prototype/ThirdPerson/Blueprints/ProtoBP_ThirdPersonCharacter.ProtoBP_ThirdPersonCharacter_C|GetCurrentItem _array_element)))
      (:3
        (Utilities|Array|Add (Variables|Players|GetPlayer4_ItemsSlots) (Variables|/Game/Prototype/ThirdPerson/Blueprints/ProtoBP_ThirdPersonCharacter.ProtoBP_ThirdPersonCharacter_C|GetCurrentItem _array_element))))))

(event Custom|OnAudioFinished_Event
  ;[0.7396 0.1521 0 0.5 60] MUSIQUE
  (bind _newparam (CallFunction|PlayRandomMusic))
  (EventDispatchers|AssignOnAudioFinished _newparam (delegate Custom|OnAudioFinished_Event)))

(event EventInit
  ;[0.7396 0.1521 0 0.5 60] MUSIQUE
  (Utilities|FlowControl|Delay 0.06)
  (bind _newparam (CallFunction|PlayRandomMusic)))

(fn PlayRandomMusic
  (bind _musiclist (Variables|Audio|GetMusicList))
  (bind _returnvalue (Utilities|Array|Length _musiclist))
  (if (> _returnvalue 0)
    (bind _output_get (Variables|Audio|SetCurrentMusicIndex (Math|Random|RandomIntegerinRange 0 (- _returnvalue 1))))
    (bind _returnvalue_2 (Audio|SpawnSound2D (Utilities|Array|Get(acopy) (Variables|Audio|GetMusicList) _output_get) 0.2 1.0 0.0 0 true false))
    (bind _output_get_2 (Variables|Audio|SetCurrentAudioComponent _returnvalue_2))
    (return _output_get_2)))

(fn WinConditionFFA
  (for (_array_element _array_index) (Variables|Default|GetRankingPlayers)
    (if (== _array_element 3)
      (Variables|Default|SetNextRound true)
      (Utilities|Array|Clear (Variables|Players|GetPlayerHP))
      (Utilities|Array|Clear (Variables|Players|GetPlayerSpeed))
      (Utilities|Array|Clear (Variables|Players|GetPlayerDashCD))
      (Utilities|Array|Clear (Variables|Players|GetPlayer1_ItemsSlots))
      (Utilities|Array|Clear (Variables|Players|GetPlayer2_ItemsSlots))
      (Utilities|Array|Clear (Variables|Players|GetPlayer3_ItemsSlots))
      (Utilities|Array|Clear (Variables|Players|GetPlayer4_ItemsSlots))
      (Utilities|Array|Clear (Variables|Players|GetPlayers))
      (Utilities|Array|Clear (Variables|Players|GetStatsPlayers))
      (Utilities|Array|Clear (Variables|Players|GetOldStatsPlayers))
      (CallFunction|EndGame)))
  (if (Variables|Default|GetNextRound)
    (Variables|Default|SetNextRound false)
    (bind _returnvalue (UserInterface|CreateWidget "/Game/Prototype/Blueprint/UI/WBP_VictoryPoints.WBP_VictoryPoints_C"))
    (UserInterface|Viewport|AddtoViewport _returnvalue 0)
    (for _index (range 0 (- (Utilities|Array|Length (Variables|Default|GetRankingPlayers)) 1))
      (Utilities|Array|SetArrayElem (Variables|Default|GetRankingPlayers) _index 0))
    (return true)
    (else
      (bind _returnvalue_2 (UserInterface|CreateWidget "/Game/Prototype/Blueprint/UI/WBP_VictoryPoints.WBP_VictoryPoints_C"))
      (UserInterface|Viewport|AddtoViewport _returnvalue_2 0)
      (return false))))