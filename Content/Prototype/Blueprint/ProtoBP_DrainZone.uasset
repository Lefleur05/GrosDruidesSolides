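; Prototype drain zone: a rising poison hazard paired with a platform that eventually falls.
; A looping timer nudges the Plane upward, while Box overlaps toggle the poison state on ProtoBP_ThirdPersonCharacter.
; After a fixed delay, a timeline raises Parent0 in world Z.
; On completion, Color1 and Color2 call each other to flash PlatformCube between two red materials until a countdown expires, then a second timeline drops it.
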(event OnComponentBeginOverlap(Box)
  (params (OverlappedComponent :type Primitive%20Component%20Object%20Reference) (OtherActor :type Actor%20Object%20Reference) (OtherComp :type Primitive%20Component%20Object%20Reference) (OtherBodyIndex :type Integer) (bFromSweep :type Boolean) (SweepResult :type Hit%20Result%20Structure%20%28by%20ref%29))
  ;[0.15 0.15 0.15 0.5] Système Poison
  (bind _asproto_bp_third_person_character (Utilities|Casting|CastToProtoBP_ThirdPersonCharacter OtherActor))
  (Default|EnterPoison _asproto_bp_third_person_character))

(event OnComponentEndOverlap(Box)
  (params (OverlappedComponent :type Primitive%20Component%20Object%20Reference) (OtherActor :type Actor%20Object%20Reference) (OtherComp :type Primitive%20Component%20Object%20Reference) (OtherBodyIndex :type Integer))
  ;[0.15 0.15 0.15 0.5] Système Poison
  (bind _asproto_bp_third_person_character (Utilities|Casting|CastToProtoBP_ThirdPersonCharacter OtherActor))
  (Default|ExitPoison _asproto_bp_third_person_character))

(event Custom|MoveUp
  ;[0.15 0.15 0.15 0.5] Montée du poison
  (Transformation|AddRelativeLocation (Variables|Default|GetPlane) "0.000000,0.000000,0.005000" false false))

(event Custom|Color2
  (if (< (Variables|Default|GetIndexToStop) 0)
    (CallFunction|FallPlatform)
    (else
      (Math|Integer|DecrementInt (Variables|Default|GetIndexToStop)
        (:%20%20
          (Rendering|Material|SetMaterial (Variables|Default|GetPlatformCube) 0 "/Game/Material/Instances/MI_BasicRed_2.MI_BasicRed_2")
          (Utilities|FlowControl|Delay (Variables|Default|GetColorRate))
          (CallFunction|Color1))))))

(event Custom|Color1
  (if (< (Variables|Default|GetIndexToStop) 0)
    (CallFunction|FallPlatform)
    (else
      (Math|Integer|DecrementInt (Variables|Default|GetIndexToStop)
        (:%20%20
          (Rendering|Material|SetMaterial (Variables|Default|GetPlatformCube) 0 "/Game/Material/Instances/MI_BasicRed_3.MI_BasicRed_3")
          (Utilities|FlowControl|Delay (Variables|Default|GetColorRate))
          (CallFunction|Color2))))))

(event Custom|FallPlatform
  (Variables|Default|SetPlatformPos (Transformation|GetWorldLocation (Variables|Default|GetPlatformCube)))
  (bind _fall (Timeline|Timeline_0 PlayFromStart)
    (:Update
      (Transformation|SetWorldLocation (Variables|Default|GetPlatformCube) (Math|Vector|MakeVector (.x (Variables|Default|GetPlatformPos)) (.y (Variables|Default|GetPlatformPos)) (Math|Float|Lerp (.z (Variables|Default|GetPlatformPos)) -5e+02 _fall)) false false))))

(event EventBeginPlay
  ;[0.15 0.15 0.15 0.5] Montée du poison
  (Utilities|FlowControl|Sequence
    (:then_0
      (Utilities|Time|SetTimerbyEvent (delegate Custom|MoveUp) (Variables|Default|GetTickRate) true)
      (CallFunction|MoveUp))
    (:then_1
      (Utilities|FlowControl|Delay 32.0)
      (Variables|Default|SetOrignalPos (Transformation|GetWorldLocation (Variables|Default|GetParent_0)))
      (bind _alphatrack (Timeline|Timeline PlayFromStart)
        (:Update
          (Transformation|SetWorldLocation (Variables|Default|GetParent_0) (Math|Vector|MakeVector (.x (Variables|Default|GetOrignalPos)) (.y (Variables|Default|GetOrignalPos)) (Math|Float|Lerp -1.6e+03 -1.2e+03 _alphatrack)) false false))
        (:Finished
          (CallFunction|Color1))))))

(fn ConstructionScript)