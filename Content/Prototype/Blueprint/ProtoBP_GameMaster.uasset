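; Round manager for a local-multiplayer free-for-all party game.
; BeginPlay creates a local player and possessed character per PlayerStart, then shows a loading screen while temporarily flagging everyone dead.
; It then adds the life HUD and syncs stats, items and rankings through ProtoBP_PartyGameInstance, which carries them between levels.
; EndRound removes players until one remains, who dances and scores, then opens LVL_Carrousel unless the match is won.
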(event Custom|EndRound
  (params (Player :type Proto%20BP%20Third%20Person%20Character%20Object%20Reference))
  (bind _playerslists (Variables|Default|GetPlayersLists))
  (bind _playerslists_2 (Variables|Default|GetPlayersLists))
  (bind _output (Utilities|Array|Get(acopy) _playerslists))
  ;[0.9323 0.7731 0.07232 0.5 74] Terminer le round
  (Utilities|Array|RemoveItem _playerslists_2 Player)
  (if (== (Utilities|Array|Length _playerslists_2) 1)
    (Input|DisableInput _output (Game|GetPlayerController (Variables|/Game/Prototype/ThirdPerson/Blueprints/ProtoBP_ThirdPersonCharacter.ProtoBP_ThirdPersonCharacter_C|GetID_Player _output)))
    (CallFunction|Dance _output)
    (bind _asbp_party_game_instance (Utilities|Casting|CastToProtoBP_PartyGameInstance (Game|GetGameInstance)))
    (Math|Integer|IncrementInt (Utilities|Array|Get(acopy) (Variables|/Game/Prototype/Blueprint/ProtoBP_PartyGameInstance.ProtoBP_PartyGameInstance_C|GetRankingPlayers _asbp_party_game_instance) (Variables|/Game/Prototype/ThirdPerson/Blueprints/ProtoBP_ThirdPersonCharacter.ProtoBP_ThirdPersonCharacter_C|GetID_Player _output))
      (:%20%20
        (bind _nextround (Default|WinConditionFFA _asbp_party_game_instance))
        (if (not _nextround)
          (Utilities|FlowControl|Delay 6.0)
          (Game|OpenLevel(byName) "LVL_Carrousel"))))))

(event Custom|ApplyAllStats
  ;[0.3812 0.1099 0.7031 0.5 45] Appliquer les stats des joueurs
  (Variables|Default|SetActualCopy 0)
  (bind _asbp_party_game_instance (Utilities|Casting|CastToProtoBP_PartyGameInstance (Game|GetGameInstance)))
  (for (_array_element _array_index) (Variables|Default|GetPlayersLists)
    (Variables|/Game/Prototype/ThirdPerson/Blueprints/ProtoBP_ThirdPersonCharacter.ProtoBP_ThirdPersonCharacter_C|SetST_PrimaryProjectile _array_element (Utilities|Array|Get(acopy) (Variables|/Game/Prototype/Blueprint/ProtoBP_PartyGameInstance.ProtoBP_PartyGameInstance_C|GetStatsPlayers _asbp_party_game_instance) (Variables|Default|GetActualCopy)))
    (bind _result (Math|Integer|IncrementInt (Variables|Default|GetActualCopy))
      (:%20%20
        (Variables|/Game/Prototype/ThirdPerson/Blueprints/ProtoBP_ThirdPersonCharacter.ProtoBP_ThirdPersonCharacter_C|SetST_SecondaryProjectile _array_element (Utilities|Array|Get(acopy) (Variables|/Game/Prototype/Blueprint/ProtoBP_PartyGameInstance.ProtoBP_PartyGameInstance_C|GetStatsPlayers _asbp_party_game_instance) _result))
        (bind _result_2 (Math|Integer|IncrementInt (Variables|Default|GetActualCopy))
          (:%20%20
            (Variables|/Game/Prototype/ThirdPerson/Blueprints/ProtoBP_ThirdPersonCharacter.ProtoBP_ThirdPersonCharacter_C|SetST_UtilitaryProjectile _array_element (Utilities|Array|Get(acopy) (Variables|/Game/Prototype/Blueprint/ProtoBP_PartyGameInstance.ProtoBP_PartyGameInstance_C|GetStatsPlayers _asbp_party_game_instance) _result_2))
            (bind _result_3 (Math|Integer|IncrementInt (Variables|Default|GetActualCopy))
              (:%20%20
                (Variables|/Game/Prototype/ThirdPerson/Blueprints/ProtoBP_ThirdPersonCharacter.ProtoBP_ThirdPersonCharacter_C|SetST_UltimateProjectile _array_element (Utilities|Array|Get(acopy) (Variables|/Game/Prototype/Blueprint/ProtoBP_PartyGameInstance.ProtoBP_PartyGameInstance_C|GetStatsPlayers _asbp_party_game_instance) _result_3))
                (Math|Integer|IncrementInt (Variables|Default|GetActualCopy)
                  (:%20%20
                    (Variables|/Script/Engine.CharacterMovementComponent|SetMaxWalkSpeed (Variables|/Script/Engine.Character|GetCharacterMovement _array_element) (Utilities|Array|Get(acopy) (Variables|/Game/Prototype/Blueprint/ProtoBP_PartyGameInstance.ProtoBP_PartyGameInstance_C|GetPlayerSpeed _asbp_party_game_instance) _array_index))
                    (bind _output_get (Variables|/Game/Prototype/ThirdPerson/Blueprints/ProtoBP_ThirdPersonCharacter.ProtoBP_ThirdPersonCharacter_C|SetMax_HealthPoints _array_element (Utilities|Array|Get(acopy) (Variables|/Game/Prototype/Blueprint/ProtoBP_PartyGameInstance.ProtoBP_PartyGameInstance_C|GetPlayerHP _asbp_party_game_instance) _array_index)))
                    (Variables|/Game/Prototype/ThirdPerson/Blueprints/ProtoBP_ThirdPersonCharacter.ProtoBP_ThirdPersonCharacter_C|SetHealthPoints _array_element _output_get)
                    (Variables|/Game/Prototype/ThirdPerson/Blueprints/ProtoBP_ThirdPersonCharacter.ProtoBP_ThirdPersonCharacter_C|SetDashCooldown _array_element (Utilities|Array|Get(acopy) (Variables|/Game/Prototype/Blueprint/ProtoBP_PartyGameInstance.ProtoBP_PartyGameInstance_C|GetPlayerDashCD _asbp_party_game_instance) _array_index))
                    (switch int _array_index
                      (:0
                        (Variables|/Game/Prototype/ThirdPerson/Blueprints/ProtoBP_ThirdPersonCharacter.ProtoBP_ThirdPersonCharacter_C|SetItemsSlots _array_element (Variables|/Game/Prototype/Blueprint/ProtoBP_PartyGameInstance.ProtoBP_PartyGameInstance_C|GetPlayer1_ItemsSlots _asbp_party_game_instance)))
                      (:1
                        (Variables|/Game/Prototype/ThirdPerson/Blueprints/ProtoBP_ThirdPersonCharacter.ProtoBP_ThirdPersonCharacter_C|SetItemsSlots _array_element (Variables|/Game/Prototype/Blueprint/ProtoBP_PartyGameInstance.ProtoBP_PartyGameInstance_C|GetPlayer2_ItemsSlots _asbp_party_game_instance)))
                      (:2
                        (Variables|/Game/Prototype/ThirdPerson/Blueprints/ProtoBP_ThirdPersonCharacter.ProtoBP_ThirdPersonCharacter_C|SetItemsSlots _array_element (Variables|/Game/Prototype/Blueprint/ProtoBP_PartyGameInstance.ProtoBP_PartyGameInstance_C|GetPlayer3_ItemsSlots _asbp_party_game_instance)))
                      (:3
                        (Variables|/Game/Prototype/ThirdPerson/Blueprints/ProtoBP_ThirdPersonCharacter.ProtoBP_ThirdPersonCharacter_C|SetItemsSlots _array_element (Variables|/Game/Prototype/Blueprint/ProtoBP_PartyGameInstance.ProtoBP_PartyGameInstance_C|GetPlayer4_ItemsSlots _asbp_party_game_instance))))))))))))))

(event Custom|LoadingScreen
  (bind _returnvalue (UserInterface|CreateWidget "/Game/Prototype/Blueprint/UI/WBP_LoadingScreen.WBP_LoadingScreen_C"))
  (UserInterface|Viewport|AddtoViewport _returnvalue 0)
  (for _array_element (Variables|Default|GetPermaPlayerLists)
    (Variables|/Game/Prototype/ThirdPerson/Blueprints/ProtoBP_ThirdPersonCharacter.ProtoBP_ThirdPersonCharacter_C|SetisDead? _array_element true))
  (Utilities|FlowControl|Delay 3.0)
  (Widget|RemovefromParent _returnvalue)
  (for _array_element_2 (Variables|Default|GetPermaPlayerLists)
    (Variables|/Game/Prototype/ThirdPerson/Blueprints/ProtoBP_ThirdPersonCharacter.ProtoBP_ThirdPersonCharacter_C|SetisDead? _array_element_2 false))
  (CallFunction|AddUIinGame))

(event Custom|Add%20UI%20In%20Game
  (bind _permaplayerlists (Variables|Default|GetPermaPlayerLists))
  ;[0.15 0.15 0.15 0.5 74] Système de spawn des joueurs / Création d'une liste des joueurs
  ;;[0.7031 0.7031 0.7031 0.5] Ajouter l'UI de jeu
  (bind _returnvalue (UserInterface|CreateWidget "/Game/Prototype/Blueprint/UI/WBP_PlayerLife.WBP_PlayerLife_C"))
  (bind _output_get (Variables|Default|SetWidgetPlayerLife _returnvalue))
  (UserInterface|Viewport|AddtoViewport _output_get 0)
  (bind _asbp_party_game_instance (Utilities|Casting|CastToProtoBP_PartyGameInstance (Game|GetGameInstance)))
  (Default|SaveStats _asbp_party_game_instance _permaplayerlists)
  (CallFunction|ApplyAllStats)
  (Default|BaseRankPlayers _asbp_party_game_instance _permaplayerlists))

(event EventBeginPlay
  (bind _returnvalue (Game|GetPlayerController 0))
  ;[0.15 0.15 0.15 0.5 74] Système de spawn des joueurs / Création d'une liste des joueurs
  ;;[0.8385 0.8385 0.8385 0.5] Récupérer la position et l'index des joueurs 1 par 1
  (bind _outactors (Actor|GetAllActorsOfClass "/Script/Engine.PlayerStart"))
  (for (_array_element _array_index) _outactors
    (bind _output_get (Variables|Default|SetArrayIndex _array_index))
    (Variables|Default|SetSpawn_Transform (Transformation|GetActorTransform _array_element))
    (bind _returnvalue_2 (Class|GameplayStatics|CreatePlayer _output_get))
    (bind _output_get_2 (Variables|Default|SetRefController _returnvalue_2))
    (if (> (Variables|Default|GetArrayIndex) 0)
      (Utilities|IsValid _output_get_2
        (:Is%20Valid
          ;;[0.4348 0.09284 0.09284 0.5] Pour les autres joueurs
          (Input|AddMappingContext (PlayerController|LocalPlayerSubsystems|GetEnhancedInputLocalPlayerSubsystem _output_get_2) "/Game/Input/IMC_Default.IMC_Default" (Variables|Default|GetArrayIndex) "(bIgnoreAllPressedKeysUntilRelease=True,bForceImmediately=False,bNotifyUserSettings=False)")
          (bind _returnvalue_3 (Game|SpawnActorfromClass "/Game/Prototype/ThirdPerson/Blueprints/ProtoBP_ThirdPersonCharacter.ProtoBP_ThirdPersonCharacter_C" (Variables|Default|GetSpawn_Transform) "Undefined" "MultiplyWithRoot" 0 0))
          (Variables|/Game/Prototype/ThirdPerson/Blueprints/ProtoBP_ThirdPersonCharacter.ProtoBP_ThirdPersonCharacter_C|SetRef_PlayerController _returnvalue_3 _output_get_2)
          (Variables|/Game/Prototype/ThirdPerson/Blueprints/ProtoBP_ThirdPersonCharacter.ProtoBP_ThirdPersonCharacter_C|SetID_Player _returnvalue_3 (Variables|Default|GetArrayIndex))
          (Pawn|Possess _output_get_2 _returnvalue_3)
          (Utilities|Array|AddUnique (Variables|Default|GetPlayersLists) _returnvalue_3)
          (Utilities|Array|AddUnique (Variables|Default|GetPermaPlayerLists) _returnvalue_3))
        (:Is%20Not%20Valid
          ;;[0.05217 0.7292 0.2087 0.5] Si le Controller existe déjà
          (Input|AddMappingContext (PlayerController|LocalPlayerSubsystems|GetEnhancedInputLocalPlayerSubsystem (Game|GetPlayerController (Variables|Default|GetArrayIndex))) "/Game/Input/IMC_Default.IMC_Default" (Variables|Default|GetArrayIndex) "(bIgnoreAllPressedKeysUntilRelease=True,bForceImmediately=False,bNotifyUserSettings=False)")
          (bind _returnvalue_4 (Game|SpawnActorfromClass "/Game/Prototype/ThirdPerson/Blueprints/ProtoBP_ThirdPersonCharacter.ProtoBP_ThirdPersonCharacter_C" (Variables|Default|GetSpawn_Transform) "Undefined" "MultiplyWithRoot" 0 0))
          (Variables|/Game/Prototype/ThirdPerson/Blueprints/ProtoBP_ThirdPersonCharacter.ProtoBP_ThirdPersonCharacter_C|SetRef_PlayerController _returnvalue_4 (Game|GetPlayerController (Variables|Default|GetArrayIndex)))
          (Variables|/Game/Prototype/ThirdPerson/Blueprints/ProtoBP_ThirdPersonCharacter.ProtoBP_ThirdPersonCharacter_C|SetID_Player _returnvalue_4 (Variables|Default|GetArrayIndex))
          (Pawn|Possess (Game|GetPlayerController (Variables|Default|GetArrayIndex)) _returnvalue_4)
          (Utilities|Array|AddUnique (Variables|Default|GetPlayersLists) _returnvalue_4)
          (Utilities|Array|AddUnique (Variables|Default|GetPermaPlayerLists) _returnvalue_4)))
      (else
        ;;[0.07724 0.196 0.8177 0.5] Pour le joueur 1
        (Input|AddMappingContext (PlayerController|LocalPlayerSubsystems|GetEnhancedInputLocalPlayerSubsystem _returnvalue) "/Game/Input/IMC_Default.IMC_Default" 0 "(bIgnoreAllPressedKeysUntilRelease=True,bForceImmediately=False,bNotifyUserSettings=False)")
        (bind _returnvalue_5 (Game|SpawnActorfromClass "/Game/Prototype/ThirdPerson/Blueprints/ProtoBP_ThirdPersonCharacter.ProtoBP_ThirdPersonCharacter_C" (Variables|Default|GetSpawn_Transform) "Undefined" "MultiplyWithRoot" 0 0))
        (Variables|/Game/Prototype/ThirdPerson/Blueprints/ProtoBP_ThirdPersonCharacter.ProtoBP_ThirdPersonCharacter_C|SetID_Player _returnvalue_5 (Variables|Default|GetArrayIndex))
        (Variables|/Game/Prototype/ThirdPerson/Blueprints/ProtoBP_ThirdPersonCharacter.ProtoBP_ThirdPersonCharacter_C|SetRef_PlayerController _returnvalue_5 _returnvalue)
        (Pawn|Possess _returnvalue _returnvalue_5)
        (Utilities|Array|AddUnique (Variables|Default|GetPlayersLists) _returnvalue_5)
        (Utilities|Array|AddUnique (Variables|Default|GetPermaPlayerLists) _returnvalue_5))))
  (CallFunction|LoadingScreen))

(fn ConstructionScript)

(fn Dance
  (params (Dancer :type Proto%20BP%20Third%20Person%20Character%20Object%20Reference))
  (bind _mesh (Variables|/Script/Engine.Character|GetMesh Dancer))
  (switch int (Math|Random|RandomIntegerinRange 0 3)
    (:0
      (Components|Animation|PlayAnimation _mesh "/Game/Prototype/Characters/Mannequins/Anims/Chicken_Dance1.Chicken_Dance1" true))
    (:1
      (Components|Animation|PlayAnimation _mesh "/Game/Prototype/Characters/Mannequins/Anims/Dancing_Twerk1.Dancing_Twerk1" true))
    (:2
      (Components|Animation|PlayAnimation _mesh "/Game/Prototype/Characters/Mannequins/Anims/Hip_Hop_Dancing1.Hip_Hop_Dancing1" true))
    (:3
      (Components|Animation|PlayAnimation _mesh "/Game/Prototype/Characters/Mannequins/Anims/House_Dancing1.House_Dancing1" true))))